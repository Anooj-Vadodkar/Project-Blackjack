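; Test dealer actor that reacts when the player chats, questions or mocks it, printing a line and changing its 2D animation state.
; Each reaction sets the DealerState enum, and a shared retriggerable delay then switches it to a common state.
; UpdateAnimation uses the enum name as a Data Table row key, then either plays a Paper2D flipbook or sets a static sprite.
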(event Custom|Chat%20To%20Player
  (Development|PrintString "Dealer: Greetings" true true "(R=0.034283,G=1.000000,B=0.000000,A=1.000000)")
  (CallFunction|Set/UpdateAnim "NewEnumerator2")
  (Utilities|FlowControl|RetriggerableDelay 3.0)
  (CallFunction|Set/UpdateAnim "NewEnumerator0"))

(event Custom|Update%20Animation
  (bind _returnvalue (Utilities|GetDataTableRow (Variables|Default|GetData%20Table) (Utilities|String|StringToName (Utilities|String|EnumtoString (Variables|Default|GetDealer%20State))))
    (:then
      (bind _output_get (Variables|Default|SetData%20Table%20Struct _returnvalue))
      (Utilities|FlowControl|Sequence
        (:then_0
          (bind _output_get_2 (Variables|Default|SetAnimated? (.Animated? (Utilities|Struct|BreakStruct_DealerAnim _output_get))))
          (if _output_get_2
            (|SetFlipbook/AnimNodes)
            (else
              (Rendering|Components|Sprite|SetSprite (Variables|Default|GetPaperSprite) (Utilities|Struct|BreakStruct_DealerAnim (Variables|Default|GetData%20Table%20Struct)))
              (Development|PrintString (Utilities|String|EnumtoString (Variables|Default|GetDealer%20State)) true true "(R=0.000000,G=0.155926,B=0.130136,A=1.000000)"))))
        (:then_1
          (Variables|Default|SetLoop? (.Loop? (Utilities|Struct|BreakStruct_DealerAnim _output_get))))))
    (:RowNotFound
      (Development|PrintString "Not Found! 
(Actor_Dealer_Test)" true true "(R=1.000000,G=0.008232,B=0.000000,A=1.000000)"))))

(event Custom|Questioned%20By%20Player
  (Development|PrintString "Dealer: Not quite sure...")
  (CallFunction|Set/UpdateAnim "NewEnumerator1")
  (Utilities|FlowControl|RetriggerableDelay 3.0)
  (CallFunction|Set/UpdateAnim "NewEnumerator0"))

(event Custom|Mocked%20By%20Player
  (Development|PrintString "Dealer: While your Jordon's are Fake..." true true "(R=1.000000,G=0.000000,B=0.015653,A=1.000000)")
  (CallFunction|Set/UpdateAnim "NewEnumerator3")
  (Utilities|FlowControl|RetriggerableDelay 3.0)
  (CallFunction|Set/UpdateAnim "NewEnumerator0"))

(fn ConstructionScript)

(fn Set/UpdateAnim
  (params (Dealer%20State :type Enum_DealerState%20Enum :default "NewEnumerator0"))
  (Variables|Default|SetDealer%20State Dealer%20State)
  (CallFunction|UpdateAnimation))