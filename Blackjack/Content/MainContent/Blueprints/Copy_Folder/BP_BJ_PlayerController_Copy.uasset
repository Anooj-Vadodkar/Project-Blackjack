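; Player controller for a copy of the Blackjack mode that drives a test dealer actor through hard-coded key bindings.
; BeginPlay caches the Blackjack game mode, prints a debug message and finds the dealer actor in the level.
; Right mouse makes the dealer chat to the player, re-finding the actor if its reference is invalid.
; Number keys 1–6 set the dealer's state enum and refresh its animation.
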(event EventBeginPlay
  (bind _asgm_blackjack_copy (Utilities|Casting|CastToGM_Blackjack_Copy (Game|GetGameMode)))
  (Variables|Default|SetGM%20Copy _asgm_blackjack_copy)
  (Development|PrintString "PC Copy: Sup Foo!" true true "(R=1.000000,G=0.000000,B=0.040611,A=1.000000)")
  (Variables|Default|GetActor%20Dealer%20Ref ; If Valid Already,\nDon't Get Again.
    (:then)
    (:else
      (bind _returnvalue (Actor|GetActorOfClass "/Game/MainContent/Blueprints/Actor_Dealer_Test.Actor_Dealer_Test_C"))
      (Variables|Default|SetActor%20Dealer%20Ref _returnvalue))))

(event Input|MouseEvents|RightMouseButton
  (params (Key :type Key%20Structure :default "None"))
  (:Pressed
    (CallFunction|TalktoDealer)))

(event Input|KeyboardEvents|4
  (params (Key :type Key%20Structure :default "None"))
  (:Pressed
    (CallFunction|Set/UpdateDealerAnim "NewEnumerator3")))

(event Input|KeyboardEvents|1
  (params (Key :type Key%20Structure :default "None"))
  (:Pressed
    (CallFunction|Set/UpdateDealerAnim "NewEnumerator0")))

(event Input|KeyboardEvents|2
  (params (Key :type Key%20Structure :default "None"))
  (:Pressed
    (CallFunction|Set/UpdateDealerAnim "NewEnumerator1")))

(event Input|KeyboardEvents|3
  (params (Key :type Key%20Structure :default "None"))
  (:Pressed
    (CallFunction|Set/UpdateDealerAnim "NewEnumerator2")))

(event Input|KeyboardEvents|6
  (params (Key :type Key%20Structure :default "None"))
  (:Pressed
    (CallFunction|Set/UpdateDealerAnim "NewEnumerator5")))

(event Input|KeyboardEvents|5
  (params (Key :type Key%20Structure :default "None"))
  (:Pressed
    (CallFunction|Set/UpdateDealerAnim "NewEnumerator4")))

(fn ConstructionScript)

(fn TalktoDealer
  (Variables|Default|GetActor%20Dealer%20Ref ; If Valid Already,\nDon't Get Again.
    (:then
      _)
    (:else
      (bind _returnvalue (Actor|GetActorOfClass "/Game/MainContent/Blueprints/Actor_Dealer_Test.Actor_Dealer_Test_C"))
      (bind _output_get (Variables|Default|SetActor%20Dealer%20Ref _returnvalue))))
  (Default|ChattoPlayer _output_get))

(fn Set/UpdateDealerAnim
  (params (Dealer%20State :type Enum_DealerState%20Enum :default "NewEnumerator0"))
  (bind _actor_dealer_ref (Variables|Default|GetActor%20Dealer%20Ref))
  (Variables|/Game/MainContent/Blueprints/Actor_Dealer_Test.Actor_Dealer_Test_C|SetDealer%20State _actor_dealer_ref Dealer%20State)
  (Default|UpdateAnimation _actor_dealer_ref))