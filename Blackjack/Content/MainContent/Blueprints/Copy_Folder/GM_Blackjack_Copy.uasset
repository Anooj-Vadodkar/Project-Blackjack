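; Blackjack game mode (a copy) that sets up the main HUD and draws random cards from a data table.
; BeginPlay casts to the copied player controller, then creates and adds the main HUD widget to the viewport.
; GetCardsDataTable picks a random card enum, uses its name as the data table row key, stores the row struct and prints its fields for debugging.
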(event Custom|Event%20Get%20Cards%20Data%20Table
  (CallFunction|GetCardsDataTable) ; I think should get randomized card "sprites"\nafter this function.
)

(event EventBeginPlay
  (bind _asbp_bj_player_controller_copy (Utilities|Casting|CastToBP_BJ_PlayerController_Copy (Game|GetPlayerController 0)))
  (bind _output_get (Variables|Default|SetPC%20Copy%20Ref _asbp_bj_player_controller_copy))
  (bind _returnvalue (UserInterface|CreateWidget "/Game/MainContent/Widgets/W_MainHUD.W_MainHUD_C" _output_get))
  (bind _output_get_2 (Variables|References|SetMain%20HUD%20Ref _returnvalue))
  (UserInterface|Viewport|AddtoViewport _output_get_2 0))

(fn ConstructionScript)

(fn RandomizeEunm/Card
  (bind _output_get (Variables|Default|SetCards%20Enum (Utilities|Enum|ByteToEnumEnum_Cards (Math|Conversions|ToByte(Integer) (Math|Random|RandomIntegerinRange 0 12)))))
  (return (Utilities|String|StringToName (Utilities|String|EnumtoString _output_get))))

(fn GetCardsDataTable
  (bind _returnvalue (Utilities|GetDataTableRow (Variables|Default|GetCard%20Data%20Table) (Functions|Pure|RandomizeEunm/Card))
    (:then
      (bind _output_get (Variables|Default|SetCards%20Struct _returnvalue))
      (Development|PrintString (Utilities|String|ToString(Text) (Utilities|Text|FormatText "Card Index:{CI} 
Card Value:{CV} 
Card Enum:{CE} 
Face Down?:{FD}" (.CardIndex (Utilities|Struct|BreakStruct_Cards _output_get)) (.CardValue (Utilities|Struct|BreakStruct_Cards _output_get)) (Utilities|String|EnumtoString (.CardEnum (Utilities|Struct|BreakStruct_Cards _output_get))) (.FaceDown? (Utilities|Struct|BreakStruct_Cards _output_get))))))
    (:RowNotFound
      (Development|PrintString "Card Not Found!" true true "(R=1.000000,G=0.000000,B=0.015156,A=1.000000)" 5.0))))