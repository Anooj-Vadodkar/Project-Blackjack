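; Game mode for a blackjack prototype that creates the main HUD and handles card draws and betting.
; A card event picks a random enum value, uses its name to look up a data table row, and adds its value to the player's total.
; Totals of 21 or over print a result and reset; lower totals send the card to the HUD.
; Bet functions move a fixed stake between the player's pot and current bet.
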(event Custom|Event%20Get%20Cards%20Data%20Table
  (bind _card (CallFunction|GetCardsDataTable))
  (bind _output_get (Variables|Default|SetPlayerCardTotal (+ (Variables|Default|GetPlayerCardTotal) (Utilities|Struct|BreakStruct_Cards _card))))
  (Math|Integer|CompareInt _output_get 21
    (:>
      (Development|PrintString "You should have stayed... You lost.")
      (Variables|Default|SetPlayerCardTotal 0))
    (:==
      (Development|PrintString "You got a 21, you won!")
      (Variables|Default|SetPlayerCardTotal 0))
    (:<
      (Default|AddNewCard (Variables|References|GetMain%20HUD%20N8) (Variables|Default|GetCards%20Struct))
      (Development|PrintString (Utilities|String|ToString(Text) (Utilities|Text|FormatText "Hand Total: {HT}" (Utilities|String|ToString(Integer) (Variables|Default|GetPlayerCardTotal)))) true true "(R=0.967549,G=0.000000,B=1.000000,A=1.000000)" 5.0))))

(event EventBeginPlay
  (bind _asbp_bj_player_controller_n8 (Utilities|Casting|CastToBP_BJ_PlayerController_N8 (Game|GetPlayerController 0)))
  (bind _output_get (Variables|References|SetPlayer%20Controller%20N8 _asbp_bj_player_controller_n8))
  (bind _returnvalue (UserInterface|CreateWidget "/Game/MainContent/Widgets/Copy_N8/W_MainHUD_N8.W_MainHUD_N8_C" _output_get))
  (bind _output_get_2 (Variables|References|SetMain%20HUD%20N8 _returnvalue))
  (UserInterface|Viewport|AddtoViewport _output_get_2 0))

(fn ConstructionScript)

(fn RandomizeEunm/Card
  (bind _output_get (Variables|Default|SetCards%20Enum (Utilities|Enum|ByteToEnumEnum_Cards (Math|Conversions|ToByte(Integer) (Math|Random|RandomIntegerinRange 0 12)))))
  (return (Utilities|String|StringToName (Utilities|String|EnumtoString _output_get))))

(fn GetCardsDataTable
  (bind _returnvalue (Utilities|GetDataTableRow (Variables|Default|GetCard%20Data%20Table) (Functions|Pure|RandomizeEunm/Card))
    (:then
      (bind _output_get (Variables|Default|SetCards%20Struct _returnvalue))
      (return _output_get))
    (:RowNotFound
      (Development|PrintString "Card Not Found!" true true "(R=1.000000,G=0.000000,B=0.015156,A=1.000000)" 5.0))))

(fn AddtoBetAmount
  (params (Player's%20Current%20Pot :type Integer))
  (bind _bet_amount (Variables|Default|GetBet%20Amount))
  (if (>= Player's%20Current%20Pot _bet_amount)
    (Variables|Default|SetCurrent%20Bet (+ _bet_amount (Variables|Default|GetCurrent%20Bet)))
    (return (- Player's%20Current%20Pot (Variables|Default|GetBet%20Amount)))
    (else
      (Development|PrintString "Can't Bet 
No Money Left!!!" true true "(R=1.000000,G=0.000000,B=0.040325,A=1.000000)" 5.0))))

(fn SubtractfromBetAmount
  (params (Player's%20Current%20Pot :type Integer))
  (if (> (Variables|Default|GetCurrent%20Bet) 0)
    (Variables|Default|SetCurrent%20Bet (- (Variables|Default|GetCurrent%20Bet) (Variables|Default|GetBet%20Amount)))
    (return (+ Player's%20Current%20Pot (Variables|Default|GetBet%20Amount)) true)
    (else
      (Development|PrintString "Can't Take 
No Money Left!!!" true true "(R=1.000000,G=0.000000,B=0.040325,A=1.000000)" 5.0)
      (return 0 false))))

(fn PlayMoneyBetted
  (bind _current_bet (Variables|Default|GetCurrent%20Bet))
  (bind _bet_amount (Variables|Default|GetBet%20Amount))
  (bind _returnvalue (>= _current_bet _bet_amount))
  (if _returnvalue
    (Development|PrintString "Lets Play!")
    (else
      (Development|PrintString "Can't, No Money!" true true "(R=1.000000,G=0.000000,B=0.040325,A=1.000000)")))
  (return _returnvalue))