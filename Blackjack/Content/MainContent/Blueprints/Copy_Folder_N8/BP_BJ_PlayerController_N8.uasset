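; Player controller for a blackjack game that relays player interactions to the dealer actor and includes debug key bindings.
; Its construction script caches the blackjack game mode and finds the dealer actor.
; Talk, question and mock functions forward to the dealer, with only talk re-fetching a missing reference.
; Right mouse asks the game mode to fetch the card data table, and number keys test dealer sprite emotion animations.
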(event EventBeginPlay
  (Development|PrintString "PC N8: Sup Foo!" true true "(R=1.000000,G=0.265625,B=0.787863,A=1.000000)"))

(event Input|MouseEvents|RightMouseButton
  (params (Key :type Key%20Structure :default "None"))
  (:Pressed
    (Default|EventGetCardsDataTable (Variables|Default|GetGM%20Blackjack%20N8))))

(event Input|KeyboardEvents|4
  (params (Key :type Key%20Structure :default "None"))
  ;[1 1 1] Sprite Emotions Testing
  (:Pressed
    (Default|Set/UpdateAnim (Variables|Default|GetActor%20Dealer%20Ref) "NewEnumerator3")))

(event Input|KeyboardEvents|1
  (params (Key :type Key%20Structure :default "None"))
  ;[1 1 1] Sprite Emotions Testing
  (:Pressed
    (Default|Set/UpdateAnim (Variables|Default|GetActor%20Dealer%20Ref) "NewEnumerator0")))

(event Input|KeyboardEvents|2
  (params (Key :type Key%20Structure :default "None"))
  ;[1 1 1] Sprite Emotions Testing
  (:Pressed
    (Default|Set/UpdateAnim (Variables|Default|GetActor%20Dealer%20Ref) "NewEnumerator1")))

(event Input|KeyboardEvents|3
  (params (Key :type Key%20Structure :default "None"))
  ;[1 1 1] Sprite Emotions Testing
  (:Pressed
    (Default|Set/UpdateAnim (Variables|Default|GetActor%20Dealer%20Ref) "NewEnumerator2")))

(event Input|KeyboardEvents|6
  (params (Key :type Key%20Structure :default "None"))
  ;[1 1 1] Sprite Emotions Testing
)

(event Input|KeyboardEvents|5
  (params (Key :type Key%20Structure :default "None"))
  ;[1 1 1] Sprite Emotions Testing
)

(fn ConstructionScript
  (bind _asgm_blackjack_n8 (Utilities|Casting|CastToGM_Blackjack_N8 (Game|GetGameMode)))
  (Variables|Default|SetGM%20Blackjack%20N8 _asgm_blackjack_n8)
  (bind _returnvalue (Actor|GetActorOfClass "/Game/MainContent/Blueprints/Actor_Dealer_Test.Actor_Dealer_Test_C"))
  (Variables|Default|SetActor%20Dealer%20Ref _returnvalue))

(fn TalktoDealer
  (Variables|Default|GetActor%20Dealer%20Ref ; If Valid Already,\nDon't Get Again.
    (:then
      _)
    (:else
      (bind _returnvalue (Actor|GetActorOfClass "/Game/MainContent/Blueprints/Actor_Dealer_Test.Actor_Dealer_Test_C"))
      (bind _output_get (Variables|Default|SetActor%20Dealer%20Ref _returnvalue))))
  (Default|ChattoPlayer _output_get))

(fn QuestionDealer
  (Default|QuestionedbyPlayer (Variables|Default|GetActor%20Dealer%20Ref)))

(fn MockDealer
  (Default|MockedbyPlayer (Variables|Default|GetActor%20Dealer%20Ref)))