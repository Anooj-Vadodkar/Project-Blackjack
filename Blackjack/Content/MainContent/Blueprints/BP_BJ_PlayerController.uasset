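; Player controller for a blackjack game that tracks the player's pot and relays player actions to the dealer and game mode.
; The construction script caches both references, and BeginPlay seeds the pot from the game mode's starting value.
; Talk, question and mock functions forward to the dealer, while bet functions update the pot only when the game mode approves.
; Keys 1–4 test dealer sprite emotions.
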(event EventBeginPlay
  (Development|PrintString "PlayerController: Hello")
  (Variables|Default|SetCurrent%20Pot (Variables|/Game/MainContent/Blueprints/GM_Blackjack.GM_Blackjack_C|GetStarting%20Pot (Variables|Default|GetGM%20Blackjack%20Ref))))

(event Input|KeyboardEvents|4
  (params (Key :type Key%20Structure :default "None"))
  ;[1 1 1] Sprite Emotions Testing
  (:Pressed
    (Default|Set/UpdateAnim (Variables|Default|GetActor%20Dealer%20Ref) "NewEnumerator3")))

(event Input|KeyboardEvents|1
  (params (Key :type Key%20Structure :default "None"))
  ;[1 1 1] Sprite Emotions Testing
  (:Pressed
    (Default|Set/UpdateAnim (Variables|Default|GetActor%20Dealer%20Ref) "NewEnumerator0")))

(event Input|KeyboardEvents|2
  (params (Key :type Key%20Structure :default "None"))
  ;[1 1 1] Sprite Emotions Testing
  (:Pressed
    (Default|Set/UpdateAnim (Variables|Default|GetActor%20Dealer%20Ref) "NewEnumerator1")))

(event Input|KeyboardEvents|3
  (params (Key :type Key%20Structure :default "None"))
  ;[1 1 1] Sprite Emotions Testing
  (:Pressed
    (Default|Set/UpdateAnim (Variables|Default|GetActor%20Dealer%20Ref) "NewEnumerator2")))

(event Input|KeyboardEvents|6
  (params (Key :type Key%20Structure :default "None"))
  ;[1 1 1] Sprite Emotions Testing
)

(event Input|KeyboardEvents|5
  (params (Key :type Key%20Structure :default "None"))
  ;[1 1 1] Sprite Emotions Testing
)

(fn ConstructionScript
  (bind _asgm_blackjack (Utilities|Casting|CastToGM_Blackjack (Game|GetGameMode)))
  (Variables|Default|SetGM%20Blackjack%20Ref _asgm_blackjack)
  (bind _returnvalue (Actor|GetActorOfClass "/Game/MainContent/Blueprints/Actor_Dealer_Test.Actor_Dealer_Test_C"))
  (Variables|Default|SetActor%20Dealer%20Ref _returnvalue))

(fn TalktoDealer
  (Variables|Default|GetActor%20Dealer%20Ref ; If Valid Already,\nDon't Get Again.
    (:then
      _)
    (:else
      (bind _returnvalue (Actor|GetActorOfClass "/Game/MainContent/Blueprints/Actor_Dealer_Test.Actor_Dealer_Test_C"))
      (bind _output_get (Variables|Default|SetActor%20Dealer%20Ref _returnvalue))))
  (Default|ChattoPlayer _output_get))

(fn QuestionDealer
  (Default|QuestionedbyPlayer (Variables|Default|GetActor%20Dealer%20Ref)))

(fn MockDealer
  (Default|MockedbyPlayer (Variables|Default|GetActor%20Dealer%20Ref)))

(fn AddMoneyBetted
  (bind (_subtract_player_s_pot _can_bet_) (Default|AddtoBetAmount (Variables|Default|GetGM%20Blackjack%20Ref) (Variables|Default|GetCurrent%20Pot)))
  (if _can_bet_
    (Variables|Default|SetCurrent%20Pot _subtract_player_s_pot)))

(fn SubtractMoneyBetted
  (bind (_return_add_player_s_pot _can_return_) (Default|SubtractfromBetAmount (Variables|Default|GetGM%20Blackjack%20Ref) (Variables|Default|GetCurrent%20Pot)))
  (if _can_return_ ; so that the player's pot don't get set to 0 somehow
    (Variables|Default|SetCurrent%20Pot _return_add_player_s_pot)))