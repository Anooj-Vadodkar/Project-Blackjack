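; Blackjack game mode that creates the main HUD and handles drawing cards for the player's hand.
; Each draw converts a random enum value to a row name, looks up that card in a DataTable and adds its value to the running total.
; Totals under 21 add the card to the HUD, while exactly 21 or a bust prints the result, resets the total and clears the hand.
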(event Custom|Event%20Get%20Cards%20Data%20Table
  (bind _card (CallFunction|GetCardsDataTable)) ; I think should get randomized card "sprites"\nafter this function.
  (bind _output_get (Variables|Default|SetPlayerCardTotal (+ (Variables|Default|GetPlayerCardTotal) (Utilities|Struct|BreakStruct_Cards _card))))
  (Math|Integer|CompareInt _output_get 21
    (:>
      (Development|PrintString "You should have stayed... You lost.")
      (Variables|Default|SetPlayerCardTotal 0)
      (Default|ClearHand (Variables|References|GetMain%20HUD%20Ref) :!label _label))
    (:==
      (Development|PrintString "You got a 21, you won!")
      (Variables|Default|SetPlayerCardTotal 0)
      (goto _label))
    (:<
      (Default|AddNewCard (Variables|References|GetMain%20HUD%20Ref) _card)
      (Development|PrintString (Utilities|String|ToString(Text) (Utilities|Text|FormatText "Hand Total: {HT}" (Utilities|String|ToString(Integer) (Variables|Default|GetPlayerCardTotal)))) true true "(R=0.967549,G=0.000000,B=1.000000,A=1.000000)" 5.0))))

(event EventBeginPlay
  (bind _asbp_bj_player_controller (Utilities|Casting|CastToBP_BJ_PlayerController (Game|GetPlayerController 0)))
  (bind _output_get (Variables|References|SetPlayer%20Controller%20Ref _asbp_bj_player_controller))
  (bind _returnvalue (UserInterface|CreateWidget "/Game/MainContent/Widgets/W_MainHUD.W_MainHUD_C" _output_get))
  (bind _output_get_2 (Variables|References|SetMain%20HUD%20Ref _returnvalue))
  (UserInterface|Viewport|AddtoViewport _output_get_2 0))

(fn ConstructionScript)

(fn RandomizeEunm/Card
  (bind _output_get (Variables|Default|SetCards%20Enum (Utilities|Enum|ByteToEnumEnum_Cards (Math|Conversions|ToByte(Integer) (Math|Random|RandomIntegerinRange 0 12)))))
  (return (Utilities|String|StringToName (Utilities|String|EnumtoString _output_get))))

(fn GetCardsDataTable
  (bind _returnvalue (Utilities|GetDataTableRow (Variables|Default|GetCard%20Data%20Table) (Functions|Pure|RandomizeEunm/Card))
    (:then
      (bind _output_get (Variables|Default|SetCards%20Struct _returnvalue))
      (return _output_get))
    (:RowNotFound
      (Development|PrintString "Card Not Found!" true true "(R=1.000000,G=0.000000,B=0.015156,A=1.000000)" 5.0))))